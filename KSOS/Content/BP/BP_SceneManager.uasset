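; Scene manager that runs one patient's dialogue encounter, from animated arrival to closing lines.
; LancementScene loads patient lines and replies from two data tables, then spawns a BP_Wankul moved by a timeline that also triggers the greeting widget and random sound.
; When the timeline finishes, it spawns BP_MoralManager and LancerScene fills the dialog widget with a line and four replies.
; Fin shows timed closing lines, adds score to the GameInstance and opens Ressource_Level.
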(event `LancementScene`
  (params (CurrentScene :type "DataTable Object Reference") (CurrentSceneAW :type "DataTable Object Reference"))
  (bind _introwidget (`self.IntroWidget`))
  (bind _ligne (`self.Ligne`))
  (bind (_output_patient _output_texte _output_membervar_19) (break `/Game/Structure/STRUCT_KSOS` (`|GetArrayItem` (`self.Tableau`))))
  (bind (_patient _texte) (break `/Game/Structure/STRUCT_KSOS` (`|GetArrayItem` (`self.Tableau`) _ligne)))
  (bind _outrownames (`DataTableFunctionLibrary.GetDataTableRowNames` CurrentScene))
  (for _array_element _outrownames
    (bind _returnvalue (`|GetDataTableRow` CurrentScene _array_element)
      (:`then`
        (`KismetArrayLibrary.Array_Add` (`self.Tableau`) _returnvalue))))
  (bind _outrownames_2 (`DataTableFunctionLibrary.GetDataTableRowNames` CurrentSceneAW))
  (for _array_element_2 _outrownames_2
    (bind _returnvalue_2 (`|GetDataTableRow` CurrentSceneAW _array_element_2)
      (:`then`
        (`KismetArrayLibrary.Array_Add` (`self.TableauAS`) _returnvalue_2))))
  (bind _returnvalue_3 (`|SpawnActorFromClass` "/Game/BP/BP_Wankul.BP_Wankul_C" (`self.GetTransform`) "Undefined" "OverrideRootScale" null null))
  (bind _output_get (set `self.CurrentWankul` _returnvalue_3))
  (`/Game/BP/BP_Wankul.InitWankul` _output_get _output_membervar_19)
  (bind _asgame_instance_bp (cast `/Game/Structure/GameInstance_BP` (`GameplayStatics.GetGameInstance`)))
  (set `/Game/Structure/GameInstance_BP.LastScore` (`/Game/Structure/GameInstance_BP.Score` _asgame_instance_bp) _asgame_instance_bp)
  (bind (_direction _transx _transy _transz _rotx _roty _rotz _scalex _scaley _scalez) (`Timeline|Timeline_0`)
    (:`Update`
      (`self.K2_SetActorTransform` _output_get (`KismetMathLibrary.MakeTransform` (`KismetMathLibrary.MakeVector` _transx _transy _transz) (`KismetMathLibrary.MakeRotator` _rotx _roty _rotz) (`KismetMathLibrary.MakeVector` _scalex _scaley _scalez)) false false))
    (:`Finished`
      (bind _returnvalue_4 (`|SpawnActorFromClass` "/Game/BP/BP_MoralManager.BP_MoralManager_C" (`self.GetTransform`) "Undefined" "OverrideRootScale" null null))
      (set `self.MoralManager` _returnvalue_4)
      (`self.lancerIntro`))
    (:`TrackDialog`
      (bind _returnvalue_5 (`|CreateWidget` "/Game/Widgets/UI_Widgets/Bonjour_Widget.Bonjour_Widget_C"))
      (bind _output_get_2 (set `self.IntroWidget` _returnvalue_5))
      (switch `int` (`KismetMathLibrary.RandomInteger` 2)
        (:`0`
          (set `self.Sound` "/Game/Sons/ahhh-homme.ahhh-homme"))
        (:`1`
          (set `self.Sound` "/Game/Sons/ahhh-homme3.ahhh-homme3"))
        (:`2`
          (bind _output_get_3 (set `self.Sound` "/Game/Sons/Coucou2.Coucou2"))))
      (`GameplayStatics.PlaySound2D` _output_get_3 1.0 1.0 0.0 null null)
      (`/Engine/EditorBlueprintResources/StandardMacros.IsValid` _output_get_2
        (:`Is Valid`
          (`UserWidget.AddToViewport` _output_get_2 0)
          (`/Engine/EditorBlueprintResources/StandardMacros.IsValid` _introwidget
            (:`Is Valid`
              (set `/Game/Widgets/UI_Widgets/Bonjour_Widget.Prenom` (`KismetTextLibrary.Conv_StringToText` (`|GetEnumeratorNameAsString` _patient)) _introwidget)
              (set `/Game/Widgets/UI_Widgets/Bonjour_Widget.Intro` (`KismetTextLibrary.Conv_StringToText` _texte) _introwidget)
              (set `self.Ligne` (+ _ligne 1)))))))
    (:`TrackUndoDialog`
      (`Widget.RemoveFromParent` _returnvalue_5))))

(event `lancerIntro`
  (bind _returnvalue (`|CreateWidget` "/Game/Widgets/UI_Widgets/Dialog_Widget.Dialog_Widget_C"))
  (bind _output_get (set `self.DialogWidget` _returnvalue))
  (`UserWidget.AddToViewport` _output_get 0)
  (`self.LancerScene`))

(event `InputAction|NextLine`
  (params (Key :type "Key Structure"))
  (:`Pressed`
    (if (`self.IntroFini?`)
      (`/Engine/EditorBlueprintResources/StandardMacros.IncrementInt` (`self.Ligne`)
        (:`  `
          (`Widget.RemoveFromParent` (`self.Dialogue_Solo`))
          (bind _returnvalue (`|CreateWidget` "/Game/Widgets/UI_Widgets/Dialog_Widget.Dialog_Widget_C"))
          (bind _output_get (set `self.DialogWidget` _returnvalue))
          (`UserWidget.AddToViewport` _output_get 0)
          (`self.LancerScene`)
          (`self.DisableInput` (`GameplayStatics.GetPlayerController` 0)))))))

(event `LancerScene`
  (bind _tableau (`self.Tableau`))
  (bind _ligne (`self.Ligne`))
  (bind _tableauas (`self.TableauAS`))
  (bind _dialogwidget (`self.DialogWidget`))
  (bind (_patient _texte) (break `/Game/Structure/STRUCT_KSOS` (`|GetArrayItem` _tableau _ligne)))
  (`/Engine/EditorBlueprintResources/StandardMacros.IsValid` (`self.DialogWidget`)
    (:`Is Valid`
      (if (>= _ligne (- (`KismetArrayLibrary.Array_Length` _tableau) 2))
        (`self.Fin`)
        (else
          (set `/Game/Widgets/UI_Widgets/Dialog_Widget.Nom` (`KismetTextLibrary.Conv_StringToText` (`|GetEnumeratorNameAsString` _patient)) _dialogwidget)
          (set `/Game/Widgets/UI_Widgets/Dialog_Widget.Text` (`KismetTextLibrary.Conv_StringToText` _texte) _dialogwidget)
          (if (>= (`self.ligneBis`) (`KismetArrayLibrary.Array_Length` _tableauas))
            (`self.Fin`)
            (else
              (set `/Game/Widgets/UI_Widgets/Dialog_Widget.Rep1` (`KismetTextLibrary.Conv_StringToText` (`.Texte_14_C711690444467771C8F57BBE968428BC` (break `/Game/Structure/STRUCT_KSOS` (`|GetArrayItem` _tableauas (`self.ligneBis`))))) (`self.DialogWidget`))
              (bind _result (`/Engine/EditorBlueprintResources/StandardMacros.IncrementInt` (`self.ligneBis`))
                (:`  `
                  (bind _output_get (set `self.ligneBis` _result))
                  (set `/Game/Widgets/UI_Widgets/Dialog_Widget.Rep2` (`KismetTextLibrary.Conv_StringToText` (`.Texte_14_C711690444467771C8F57BBE968428BC` (break `/Game/Structure/STRUCT_KSOS` (`|GetArrayItem` (`self.TableauAS`) _output_get)))) (`self.DialogWidget`))
                  (bind _result_2 (`/Engine/EditorBlueprintResources/StandardMacros.IncrementInt` (`self.ligneBis`))
                    (:`  `
                      (bind _output_get_2 (set `self.ligneBis` _result_2))
                      (set `/Game/Widgets/UI_Widgets/Dialog_Widget.Rep3` (`KismetTextLibrary.Conv_StringToText` (`.Texte_14_C711690444467771C8F57BBE968428BC` (break `/Game/Structure/STRUCT_KSOS` (`|GetArrayItem` (`self.TableauAS`) _output_get_2)))) (`self.DialogWidget`))
                      (bind _result_3 (`/Engine/EditorBlueprintResources/StandardMacros.IncrementInt` (`self.ligneBis`))
                        (:`  `
                          (bind _output_get_3 (set `self.ligneBis` _result_3))
                          (set `/Game/Widgets/UI_Widgets/Dialog_Widget.Rep4` (`KismetTextLibrary.Conv_StringToText` (`.Texte_14_C711690444467771C8F57BBE968428BC` (break `/Game/Structure/STRUCT_KSOS` (`|GetArrayItem` (`self.TableauAS`) _output_get_3)))) (`self.DialogWidget`))
                          (bind _result_4 (`/Engine/EditorBlueprintResources/StandardMacros.IncrementInt` (`self.ligneBis`))
                            (:`  `
                              (set `self.ligneBis` _result_4))))))))))))))))

(event `Fin`
  (bind _dialogue_solo (`self.Dialogue_Solo`))
  (`Widget.RemoveFromParent` (`self.DialogWidget`))
  (bind _returnvalue (`|CreateWidget` "/Game/Widgets/UI_Widgets/Dialog_Solo_Widget.Dialog_Solo_Widget_C"))
  (bind _output_get (set `self.Dialogue_Solo` _returnvalue))
  (`UserWidget.AddToViewport` _output_get 0)
  (set `/Game/Widgets/UI_Widgets/Dialog_Solo_Widget.Intro` (`KismetTextLibrary.Conv_StringToText` (`.Texte_14_C711690444467771C8F57BBE968428BC` (break `/Game/Structure/STRUCT_KSOS` (`|GetArrayItem` (`self.Tableau`) (`self.Ligne`))))) _dialogue_solo)
  (`KismetSystemLibrary.Delay` 2.0)
  (`Widget.RemoveFromParent` _dialogue_solo)
  (if (== (`self.Ligne`) (- (`KismetArrayLibrary.Array_Length` (`self.Tableau`)) 2))
    (set `self.Ligne` (- (`KismetArrayLibrary.Array_Length` (`self.Tableau`)) 1))
    (`self.Fin`)
    (else
      (bind _asgame_instance_bp (cast `/Game/Structure/GameInstance_BP` (`GameplayStatics.GetGameInstance`)))
      (set `/Game/Structure/GameInstance_BP.Score` (+ (`/Game/Structure/GameInstance_BP.Score` _asgame_instance_bp) 4000) _asgame_instance_bp)
      (`self.ChangerClient`))))

(event `ChangerClient`
  (`GameplayStatics.OpenLevel` "Ressource_Level"))

(fn `UserConstructionScript`)