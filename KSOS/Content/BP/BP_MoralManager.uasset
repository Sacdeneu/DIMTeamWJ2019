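; BP_MoralManager is a Blueprint that stores and adjusts a morale value.
; ResetMoral sets CurrentMoral to a given base, while AjoutMoral and SupprimerMoral add or subtract a rate, clamped at FullMoral and zero respectively.
; Its event graph and construction script are empty, so the value changes only when these functions are called.
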(event `self.ReceiveBeginPlay`)

(fn `AjoutMoral`
  (params (Rate :type Integer))
  (bind _returnvalue (+ (`self.CurrentMoral`) (`KismetMathLibrary.Conv_IntToDouble` Rate)))
  (if (<= _returnvalue (`self.FullMoral`))
    (set `self.CurrentMoral` _returnvalue)
    (else
      (set `self.CurrentMoral` (`self.FullMoral`)))))

(fn `ResetMoral`
  (params (MoralBase :type "Float (double-precision)"))
  (set `self.CurrentMoral` MoralBase))

(fn `SupprimerMoral`
  (params (Rate :type Integer))
  (bind _returnvalue (- (`self.CurrentMoral`) (`KismetMathLibrary.Conv_IntToDouble` Rate)))
  (if (>= _returnvalue 0.0)
    (set `self.CurrentMoral` _returnvalue)
    (else
      (set `self.CurrentMoral` 0.0))))

(fn `UserConstructionScript`)